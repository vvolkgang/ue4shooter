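; BP_PickableAmmo is a pickable ammo item that spins in the world and grants ammo to a ShooterCharacter.
; Tick rotates BaseMesh around its yaw axis, scaled by delta time.
; PickItem casts the pawn to ShooterCharacter and, only if CanAddAmmo passes, adds AmmoToAdd and then calls the parent pickup logic.
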(event EventBeginPlay
  (|CallParentFunction) ; This node is disabled and will not be called.\nDrag off pins to build functionality.
)

(event Collision|EventActorBeginOverlap
  (params (OtherActor :type Actor%20Object%20Reference))
  (|CallParentFunction OtherActor) ; This node is disabled and will not be called.\nDrag off pins to build functionality.
)

(event EventTick
  (params (DeltaSeconds :type Float%20%28single-precision%29))
  (|CallParentFunction DeltaSeconds)
  (Transformation|AddRelativeRotation (Variables|Default|GetBaseMesh) (Math|Rotator|MakeRotator 0.0 0.0 (* DeltaSeconds 2e+02)) false false))

(event EventPickItem
  (params (Pawn :type Actor%20Object%20Reference))
  (bind _asshooter_character (Utilities|Casting|CastToShooterCharacter Pawn))
  (if (Class|ShooterCharacter|CanAddAmmo _asshooter_character)
    (Class|ShooterCharacter|AddAmmo _asshooter_character (Variables|PickableDetails|GetAmmoToAdd))
    (|CallParentFunction 0)))

(fn ConstructionScript
  (|CallParentFunction))